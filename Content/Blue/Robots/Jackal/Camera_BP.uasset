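; Camera Blueprint for the Jackal robot that drives player view rotation and triggers robot movement between rooms.
; It zeroes control rotation on BeginPlay, then applies its Rotation variable to the player controller every Tick.
; Custom events show the RoomEndInputs widget, or construct AvailableRooms, call the Jackal's MoveToLocation and increment its Timestep; despite its name, Possesscamera possesses nothing.
; SetActivePath stores the chosen room on the Jackal and selects the matching path from TestArrayStruct.
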(event Custom|Possess%20camera
  (bind _jackal (Variables|Default|GetJackal))
  (Game|ConstructObjectfromClass "/Game/Blue/UIWidgets/AvailableRooms.AvailableRooms_C" (Game|Player|GetPlayerPawn 0))
  (Default|MovetoLocation _jackal)
  (Variables|/Game/Blue/Robots/Jackal/jackal_3d_model_Blueprint.jackal_3d_model_Blueprint_C|SetTimestep _jackal (+ (Variables|/Game/Blue/Robots/Jackal/jackal_3d_model_Blueprint.jackal_3d_model_Blueprint_C|GetTimestep _jackal) 1)))

(event Custom|show%20widget
  (bind _returnvalue (UserInterface|CreateWidget "/Game/Blue/UIWidgets/RoomEndInputs.RoomEndInputs_C" (Game|GetPlayerController 0)))
  (UserInterface|Viewport|AddtoViewport _returnvalue 0))

(event EventBeginPlay
  (Pawn|SetControlRotation (Game|GetPlayerController 0) (Math|Rotator|MakeRotator 0.0 0.0 0.0)))

(event Collision|EventActorBeginOverlap
  (params (OtherActor :type Actor%20Object%20Reference)))

(event EventTick
  (params (DeltaSeconds :type Float%20%28single-precision%29))
  (Pawn|SetControlRotation (Game|GetPlayerController 0) (Variables|Default|GetRotation)))

(fn ConstructionScript)

(fn SetActivePath
  (params (Active%20Room :type Integer))
  (bind _jackal (Variables|Default|GetJackal))
  (bind _test_array_struct (Variables|/Game/Blue/Robots/Jackal/jackal_3d_model_Blueprint.jackal_3d_model_Blueprint_C|GetTest%20Array%20Struct _jackal))
  (bind _output_get (Variables|/Game/Blue/Robots/Jackal/jackal_3d_model_Blueprint.jackal_3d_model_Blueprint_C|SetActive%20Room _jackal Active%20Room))
  (Variables|/Game/Blue/Robots/Jackal/jackal_3d_model_Blueprint.jackal_3d_model_Blueprint_C|SetActive%20Path _jackal (Utilities|Select :Index _output_get :Option%200 0 :Option%201 (.1 _test_array_struct) :Option%202 (.2 _test_array_struct) :Option%203 (.3 _test_array_struct) :Option%204 (.4 _test_array_struct) :Option%205 (.5 _test_array_struct)))
  (return))